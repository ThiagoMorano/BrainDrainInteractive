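; Weighing scale level-event prop that tilts, grows a wall-run document and moves its seal as objects are added to the dish.
; AddObjecttoWeighingDish increments an object count capped at a maximum, which sets proportional targets between initial and final values.
; Each Tick eases arm roll, document scale and seal position toward those targets using a fixed lerp alpha, independent of delta time.
; Both bowls copy their anchor components' world locations, following the arm without taking its rotation.
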(event `self.ReceiveTick`
  (params (DeltaSeconds :type "Float (single-precision)"))
  (bind _arm (`self.Arm`))
  (bind (_relativerotation_roll _relativerotation_pitch _relativerotation_yaw) (`KismetMathLibrary.BreakRotator` (`SceneComponent.RelativeRotation` _arm)))
  (bind _output_get (set `self.CurrentAngle` (`KismetMathLibrary.Lerp` (`self.CurrentAngle`) (+ (`self.InitialAngle`) (* (`self.NumObjects`) (/ (- (`self.FinalAngle`) (`self.InitialAngle`)) (`KismetMathLibrary.Conv_IntToDouble` (`self.MaxNumOfObjects`))))) (`self.SpeedOfLerp`))))
  (`SceneComponent.K2_SetRelativeRotation` _arm (`KismetMathLibrary.MakeRotator` _output_get _relativerotation_pitch _relativerotation_yaw) false false)
  (`SceneComponent.K2_SetWorldLocation` (`self.LeftBowl`) (`SceneComponent.K2_GetComponentLocation` (`self.LeftBowlPosition`)) false false)
  (`SceneComponent.K2_SetWorldLocation` (`self.RightBowl`) (`SceneComponent.K2_GetComponentLocation` (`self.RightBowlPosition`)) false false)
  (bind _output_get_2 (set `self.WallRunDocCurrenScale` (`KismetMathLibrary.VLerp` (`self.WallRunDocCurrenScale`) (+ (`self.WallRunDocumentInitialScale`) (* (/ (- (`self.WallRunDocumentFinalScale`) (`self.WallRunDocumentInitialScale`)) (`self.MaxNumOfObjects`)) (`self.NumObjects`))) (`self.SpeedOfLerp`))))
  (`SceneComponent.SetRelativeScale3D` (`self.WallRunDocument`) _output_get_2)
  (bind _output_get_3 (set `self.SealCurrentLocation` (`KismetMathLibrary.VLerp` (`self.SealCurrentLocation`) (+ (`self.SealInitialLocation`) (* (/ (- (`self.SealFinalLocation`) (`self.SealInitialLocation`)) (`self.MaxNumOfObjects`)) (`self.NumObjects`))) (`self.SpeedOfLerp`))))
  (`SceneComponent.K2_SetRelativeLocation` (`self.DocumentSeal`) _output_get_3 false false))

(event `Add Object to Weighing Dish`
  (bind _result (`/Engine/EditorBlueprintResources/StandardMacros.IncrementInt` (`self.NumObjects`))
    (:`  `
      (if (> _result (`self.MaxNumOfObjects`))
        (set `self.NumObjects` (`self.MaxNumOfObjects`))))))

(fn `UserConstructionScript`)