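; BP_Statue is a puzzle actor that assembles pushable statue parts as they enter its cylinder trigger.
; Overlapping parts lock and lerp by timeline to per-part final transforms, queuing while another arranges; startup parts snap in on BeginPlay.
; Once every part is placed, it fires its assembled call, hides the cylinder and, if a body part is assigned, moves it while rotating one statue part, apparently the left arm.
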(event `self.ReceiveBeginPlay`
  (for _array_element (`self.StartupStatueParts`)
    (`/Engine/EditorBlueprintResources/StandardMacros.IsValid` _array_element
      (:`Is Valid`
        (set `/Game/ThirdPersonBP/Blueprints/TorsoBreathing/BP_PushableObject.CanBePushed?` false _array_element)
        (`KismetArrayLibrary.Array_Add` (`self.ArrangedParts`) _array_element)
        (`self.K2_SetActorTransform` _array_element (`BlueprintMapLibrary.Map_Find` (`self.FinalTransforms`) (`/Game/ThirdPersonBP/Blueprints/TorsoBreathing/BP_PushableObject.StatuePart` _array_element)) false false)))))

(event `self.Cylinder.OnComponentBeginOverlap`
  (params (OverlappedComponent :type "PrimitiveComponent Object Reference") (OtherActor :type "Actor Object Reference") (OtherComp :type "PrimitiveComponent Object Reference") (OtherBodyIndex :type Integer) (bFromSweep :type Boolean) (SweepResult :type "HitResult Structure (by ref)"))
  (if (not (`self.Done?`))
    (bind _asbp_pushable_object (cast `/Game/ThirdPersonBP/Blueprints/TorsoBreathing/BP_PushableObject` OtherActor))
    (bind _statuepart (`/Game/ThirdPersonBP/Blueprints/TorsoBreathing/BP_PushableObject.StatuePart` _asbp_pushable_object))
    (if (`|EnumInequality` _statuepart "NewEnumerator6")
      (if (`self.Arranging?`)
        (`KismetArrayLibrary.Array_Add` (`self.Queue`) _asbp_pushable_object)
        (`/Game/ThirdPersonBP/Blueprints/TorsoBreathing/BP_PushableObject.StopMovement` _asbp_pushable_object)
        (else
          (`self.ArrangePart` _asbp_pushable_object _statuepart))))))

(event `ArrangePart`
  (params (Pushable :type "/Game/ThirdPersonBP/Blueprints/TorsoBreathing/BP_PushableObject Object Reference") (`Statue Part` :type "/Game/Misc/LevelEvents/ENUM_StatueParts Enum" :default "NewEnumerator6"))
  (bind _queue (`self.Queue`))
  (bind _output (`|GetArrayItem` _queue))
  (set `self.Arranging?` true)
  (set `/Game/ThirdPersonBP/Blueprints/TorsoBreathing/BP_PushableObject.CanBePushed?` false Pushable)
  (set `self.FinalTransform` (`BlueprintMapLibrary.Map_Find` (`self.FinalTransforms`) `Statue Part`))
  (set `self.OriginalTransform` (`self.GetTransform` Pushable))
  (bind _output_get (set `self.CurrentPushable` Pushable))
  (`KismetArrayLibrary.Array_Add` (`self.ArrangedParts`) _output_get)
  (bind (_direction _percent) (`Timeline|ArrangeTimeline` :!via `PlayFromStart`)
    (:`Update`
      (`self.K2_SetActorTransform` (`self.CurrentPushable`) (`KismetMathLibrary.TLerp` (`self.OriginalTransform`) (`self.FinalTransform`) _percent "DualQuatInterp") false false))
    (:`Finished`
      (set `self.Arranging?` false)
      (`KismetArrayLibrary.Array_RemoveItem` _queue (`self.CurrentPushable`))
      (`/Engine/EditorBlueprintResources/StandardMacros.IsValid` _output
        (:`Is Valid`
          (`self.ArrangePart` _output (`/Game/ThirdPersonBP/Blueprints/TorsoBreathing/BP_PushableObject.StatuePart` _output)))
        (:`Is Not Valid`
          (if (>= (`KismetArrayLibrary.Array_Length` (`self.ArrangedParts`)) (`BlueprintMapLibrary.Map_Length` (`self.FinalTransforms`)))
            (`self.OnEveryPartAssembled`)))))))

(event `OnEveryPartAssembled`
  (bind _bodyparttofind (`self.BodyPartToFind`))
  (`/Engine/EditorBlueprintResources/StandardMacros.DoOnce` false
    (:`Completed`
      (`self.OnAssembled`)
      (set `self.Done?` true)
      (`SceneComponent.SetVisibility` (`self.Cylinder`) false false)
      (`/Engine/EditorBlueprintResources/StandardMacros.IsValid` (`self.BodyPartToFind`)
        (:`Is Valid`
          (`PrimitiveComponent.SetCollisionResponseToAllChannels` (`/Game/ThirdPersonBP/Blueprints/BodyPartAbilities/BP_BodyPart.PickupArea` _bodyparttofind) "ECR_Ignore")
          (set `self.OriginalBodyPartTransform` (`self.GetTransform` _bodyparttofind))
          (for _array_element (`self.ArrangedParts`)
            (if (`|EnumEquality` (`/Game/ThirdPersonBP/Blueprints/TorsoBreathing/BP_PushableObject.StatuePart` _array_element) "NewEnumerator4")
              (set `self.LeftArmPart` _array_element)
              (break)))
          (set `self.OriginalRotation` (`self.K2_GetActorRotation` (`self.LeftArmPart`)))
          (`self.SetActorEnableCollision` (`self.LeftArmPart`) false)
          (set `self.FinalRot` (`KismetMathLibrary.MakeRotator` (- (.roll (`self.OriginalRotation`)) -75.0) (.pitch (`self.OriginalRotation`)) (.yaw (`self.OriginalRotation`))))
          (bind (_direction _percent _rotation) (`Timeline|NewTimeline` :!via `PlayFromStart`)
            (:`Update`
              (`self.K2_SetActorTransform` (`self.BodyPartToFind`) (`KismetMathLibrary.TLerp` (`self.OriginalBodyPartTransform`) (`self.FinalBodyPartTransform`) _percent) false false)
              (`self.K2_SetActorRotation` (`self.LeftArmPart`) (`KismetMathLibrary.RLerp` (`self.OriginalRotation`) (`self.FinalRot`) _rotation) false))
            (:`Finished`
              (`PrimitiveComponent.SetCollisionResponseToAllChannels` (`/Game/ThirdPersonBP/Blueprints/BodyPartAbilities/BP_BodyPart.PickupArea` (`self.BodyPartToFind`)) "ECR_Overlap")
              (`self.SetActorEnableCollision` (`self.LeftArmPart`) true))))))))

(fn `UserConstructionScript`)