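; Sound manager that plays music and sound effects and controls their volumes through separate sound mix class overrides.
; Music runs on one 2D component with fade-out/fade-in track transitions and timed pauses, and is paused at zero volume.
; Any requested theme track is swapped for the ThemeTracks entry matching the player's body part count.
; Effects play as one-shots, or as tracked components that StopSoundEffects fades out together.
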(event `UpdatePlayer`
  (params (NewPlayer :type "Actor Object Reference"))
  (bind _startupmusic (`self.StartUpMusic`))
  (`/Engine/EditorBlueprintResources/StandardMacros.IsValid` NewPlayer
    (:`Is Valid`
      (set `self.BodyPartCompRef` (`self.GetComponentByClass` NewPlayer "/Game/ThirdPersonBP/Blueprints/BodyPartAbilities/BpC_BodyParts.BpC_BodyParts_C")))
    (:`Is Not Valid`
      _))
  (`/Engine/EditorBlueprintResources/StandardMacros.IsValid` (`self.MusicComponent`)
    (:`Is Not Valid`
      (`/Engine/EditorBlueprintResources/StandardMacros.IsValid` _startupmusic
        (:`Is Valid`
          (if (not (`self.SurpressMusic?`))
            (`self.PlayMusic` _startupmusic)))))))

(event `PauseMusic`
  (params (FadeOut :type "Float (double-precision)") (Duration :type "Float (double-precision)"))
  (bind _musiccomponent (`self.MusicComponent`))
  (`/Engine/EditorBlueprintResources/StandardMacros.IsValid` _musiccomponent
    (:`Is Valid`
      (`AudioComponent.FadeOut` _musiccomponent FadeOut 0.0)
      (set `self.StoredSound` (`AudioComponent.Sound` _musiccomponent))
      (`KismetSystemLibrary.Delay` FadeOut)
      (`ActorComponent.K2_DestroyComponent` _musiccomponent)
      (`KismetSystemLibrary.Delay` (- Duration FadeOut))
      (bind _returnvalue (`GameplayStatics.CreateSound2D` (`self.StoredSound`) 1.0 1.0 0.0 null))
      (bind _output_get (set `self.MusicComponent` _returnvalue))
      (`AudioComponent.FadeIn` _musiccomponent FadeOut 1.0 0.0)
      (`AudioComponent.FadeIn` _output_get FadeOut 1.0 0.0))))

(event `TransitionToNewTrack`
  (params (Track :type "SoundBase Object Reference"))
  (bind _bodypartcompref (`self.BodyPartCompRef`))
  (if (not (`self.InTransition?`))
    (set `self.InTransition?` true)
    (bind _output_get (set `self.NextTrackToPlay` Track))
    (`AudioComponent.FadeOut` (`self.MusicComponent`) (`self.FadeOutDuration`) 0.0)
    (if (`KismetArrayLibrary.Array_Contains` (`self.ThemeTracks`) _output_get)
      (`/Engine/EditorBlueprintResources/StandardMacros.IsValid` _bodypartcompref
        (:`Is Valid`
          (set `self.NextTrackToPlay` (`|GetArrayItem` (`self.ThemeTracks`) (- (`BlueprintSetLibrary.Set_Length` (`/Game/ThirdPersonBP/Blueprints/BodyPartAbilities/BpC_BodyParts.GetBodyParts` _bodypartcompref)) 1))))
        (:`Is Not Valid`
          _)))
    (`KismetSystemLibrary.Delay` (* (`self.FadeOutDuration`) 1.1))
    (bind _returnvalue (`GameplayStatics.CreateSound2D` (`self.NextTrackToPlay`) 1.0 1.0 0.0 null))
    (bind _output_get_2 (set `self.MusicComponent` _returnvalue))
    (`AudioComponent.FadeIn` _output_get_2 (* (`self.FadeOutDuration`) 0.5) 1.0 0.0)
    (set `self.InTransition?` false)))

(event `StopSoundEffects`
  (params (Duration :type "Float (double-precision)" :default 1.0))
  (bind _accessibleeffects (`self.AccessibleEffects`))
  (for _array_element _accessibleeffects
    (`/Engine/EditorBlueprintResources/StandardMacros.IsValid` _array_element
      (:`Is Valid`
        (`AudioComponent.FadeOut` _array_element Duration 0.0))))
  (`KismetSystemLibrary.Delay` Duration)
  (`KismetArrayLibrary.Array_Clear` _accessibleeffects))

(fn `AdjustVolume`
  (params (`Music?` :type Boolean) (Volume :type "Float (double-precision)") (FadeInTime :type "Float (double-precision)"))
  (bind _musiccomponent (`self.MusicComponent`))
  (if `Music?`
    (bind _output_get (set `self.MusicVolume` Volume))
    (`GameplayStatics.SetSoundMixClassOverride` "/Game/Misc/Sound/SoundMix_Music.SoundMix_Music" "/Game/Misc/Sound/SoundClass_Music.SoundClass_Music" Volume 1.0 FadeInTime)
    (if (and (not (`self.SurpressMusic?`)) (not (`self.StopMusic`)) (<= _output_get 0.0))
      (set `self.StopMusic` true)
      (`/Engine/EditorBlueprintResources/StandardMacros.IsValid` _musiccomponent
        (:`Is Valid`
          (`AudioComponent.SetPaused` _musiccomponent true)))
      (elif (and (not (`self.SurpressMusic?`)) (`self.StopMusic`) (> _output_get 0.0))
        (set `self.StopMusic` false)
        (`/Engine/EditorBlueprintResources/StandardMacros.IsValid` (`self.MusicComponent`)
          (:`Is Valid`
            (`AudioComponent.SetPaused` (`self.MusicComponent`) false)))))
    (else
      (set `self.EffectsVolume` Volume)
      (`GameplayStatics.SetSoundMixClassOverride` "/Game/Misc/Sound/SoundMix_Effects.SoundMix_Effects" "/Game/Misc/Sound/SoundClass_Effects.SoundClass_Effects" Volume 1.0 FadeInTime))))

(fn `GetVolume`
  (params (`Music?` :type Boolean :default true))
  (returns (Out :type "Float (double-precision)"))
  (return (select `bool` `Music?` :`false` (`self.EffectsVolume`) :`true` (`self.MusicVolume`))))

(fn `PlayAccessibleEffect`
  (params (Effect :type "SoundBase Object Reference") (`OnLocation?` :type Boolean) (Location :type "Vector Structure") (StartTime :type "Float (double-precision)") (Pitch :type "Float (double-precision)" :default 1.0) (Volume :type "Float (double-precision)" :default 1.0))
  (bind _accessibleeffects (`self.AccessibleEffects`))
  (if `OnLocation?`
    (bind _returnvalue (`GameplayStatics.SpawnSoundAtLocation` Effect Location (struct) Volume Pitch StartTime null null))
    (`KismetArrayLibrary.Array_Add` _accessibleeffects _returnvalue)
    (else
      (bind _returnvalue_2 (`GameplayStatics.SpawnSound2D` Effect Volume Pitch StartTime null))
      (`KismetArrayLibrary.Array_Add` _accessibleeffects _returnvalue_2))))

(fn `PlayEffect`
  (params (Effect :type "SoundBase Object Reference") (`OnLocation?` :type Boolean :default true) (Location :type "Vector Structure") (StartTime :type "Float (double-precision)") (Pitch :type "Float (double-precision)" :default 1.0) (Volume :type "Float (double-precision)" :default 1.0))
  (if `OnLocation?`
    (`GameplayStatics.PlaySoundAtLocation` Effect Location (struct) Volume Pitch StartTime null null null)
    (else
      (`GameplayStatics.PlaySound2D` Effect Volume Pitch StartTime null null))))

(fn `PlayMusic`
  (params (Music :type "SoundBase Object Reference"))
  (bind _bodypartcompref (`self.BodyPartCompRef`))
  (if (not (`self.SurpressMusic?`))
    (`/Engine/EditorBlueprintResources/StandardMacros.IsValid` (`self.MusicComponent`)
      (:`Is Valid`
        (`self.TransitionToNewTrack` Music))
      (:`Is Not Valid`
        (if (`KismetArrayLibrary.Array_Contains` (`self.ThemeTracks`) Music)
          (`/Engine/EditorBlueprintResources/StandardMacros.IsValid` _bodypartcompref
            (:`Is Valid`
              (bind _returnvalue (`GameplayStatics.CreateSound2D` (`|GetArrayItem` (`self.ThemeTracks`) (- (`BlueprintSetLibrary.Set_Length` (`/Game/ThirdPersonBP/Blueprints/BodyPartAbilities/BpC_BodyParts.GetBodyParts` _bodypartcompref)) 1)) 1.0 1.0 0.0 null))
              (bind _output_get (set `self.MusicComponent` _returnvalue))
              (`AudioComponent.Play` _output_get 0.0))
            (:`Is Not Valid`
              (bind _returnvalue_2 (`GameplayStatics.CreateSound2D` Music 1.0 1.0 0.0 null :!label _label))
              (bind _output_get_2 (set `self.MusicComponent` _returnvalue_2))
              (`AudioComponent.Play` _output_get_2 0.0)))
          (else
            (goto _label)))))))

(fn `ReturnToDefaultTheme`
  (bind _startupmusic (`self.StartUpMusic`))
  (`/Engine/EditorBlueprintResources/StandardMacros.IsValid` _startupmusic
    (:`Is Valid`
      (`self.PlayMusic` _startupmusic))))

(fn `UserConstructionScript`)