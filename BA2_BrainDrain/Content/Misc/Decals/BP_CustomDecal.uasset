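; BP_CustomDecal is a placeable decal actor whose look is set per instance through texture, opacity, color and emissive variables.
; The construction script creates a dynamic material instance on the Decal component, stores it as MatInstance and writes those variables into the matching material parameters.
; It has no runtime logic, as all event graph nodes are disabled stubs.
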(fn `UserConstructionScript`
  (bind _returnvalue (`DecalComponent.CreateDynamicMaterialInstance` (`self.Decal`)))
  (bind _output_get (set `self.MatInstance` _returnvalue))
  (`MaterialInstanceDynamic.SetTextureParameterValue` _output_get "Texture" (`self.DecalTexture`))
  (`MaterialInstanceDynamic.SetScalarParameterValue` _output_get "Opacity" (`self.DecalOpacity`))
  (`MaterialInstanceDynamic.SetVectorParameterValue` _output_get "Color" (`self.DecalColor`))
  (`MaterialInstanceDynamic.SetScalarParameterValue` _output_get "EmissiveBoost" (`self.DecalEmissive`)))