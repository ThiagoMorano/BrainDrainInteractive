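; Actor component on ThirdPersonCharacter that saves and restores game progress through a BP_PlayerSaveGame slot.
; It tracks loaded streaming sublevels and per-level tag lists, saving them with player transform, control rotation, settings, found memories and collected body parts.
; Loading reuses the cached save object or reads the slot, restores that data, swaps streamed levels without blocking and teleports the player.
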(event `self.ReceiveBeginPlay`
  (bind _asthird_person_character (cast `/Game/ThirdPersonBP/Blueprints/ThirdPersonCharacter` (`self.GetOwner`))
    (:`then`
      (set `self.CharacterRef` _asthird_person_character))
    (:`CastFailed`
      (`KismetSystemLibrary.PrintString` "Error: Using incorrect character class for BpC_Saving to work!" true true (struct :`R` 1.0 :`G` 0.201192 :`A` 1.0) 5.0))))

(event `OnGameLoaded`
  (params (LevelsToUnload :type "Array of Name") (LevelsToLoad :type "Array of Name") (`Player Position` :type "Vector Structure") (`Player Rotation` :type "Rotator Structure") (`Control Rotation` :type "Rotator Structure"))
  (bind _currentlyloadedlevels (`self.CurrentlyLoadedLevels`))
  (bind _characterref (`self.CharacterRef`))
  (for _array_element LevelsToUnload
    (`GameplayStatics.UnloadStreamLevel` _array_element))
  (for _array_element_2 LevelsToLoad
    (`GameplayStatics.LoadStreamLevel` _array_element_2 true))
  (`BlueprintSetLibrary.Set_Clear` _currentlyloadedlevels)
  (`BlueprintSetLibrary.Set_AddItems` _currentlyloadedlevels LevelsToLoad)
  (`Actor.K2_SetActorLocationAndRotation` _characterref `Player Position` `Player Rotation` false true)
  (`Controller.SetControlRotation` (`Pawn.GetController` _characterref) `Control Rotation`)
  (`self.OnGameLoadedDis`))

(fn `AdjustLoadedLevels`
  (params (Level :type Name) (`Add?` :type Boolean :default true))
  (bind _currentlyloadedlevels (`self.CurrentlyLoadedLevels`))
  (if `Add?`
    (`BlueprintSetLibrary.Set_Add` _currentlyloadedlevels Level)
    (return)
    (else
      (`BlueprintSetLibrary.Set_Remove` _currentlyloadedlevels Level)
      (return))))

(fn `HasSaveGame?`
  (returns (`Out?` :type Boolean))
  (bind _returnvalue (`GameplayStatics.DoesSaveGameExist` (`self.SaveSlotName`)))
  (return _returnvalue))

(fn `HasTag?`
  (params (`Level Name` :type Name) (Tag :type String))
  (returns (`Out?` :type Boolean))
  (bind (_value _returnvalue) (`BlueprintMapLibrary.Map_Find` (`self.LevelTags`) `Level Name`))
  (if _returnvalue
    (return (`KismetArrayLibrary.Array_Contains` (`.Tags_3_AC2B457843A0A54F6BC1A799293853A6` (break `/Game/Misc/SavingAndLoading/STR_AreaTags` _value)) Tag))
    (else
      (return false))))

(fn `LoadGame`
  (bind _savegameobject (`self.SaveGameObject`))
  (bind _characterref (`self.CharacterRef`))
  (if (`self.HasSaveGame?`)
    (`/Engine/EditorBlueprintResources/StandardMacros.IsValid` (`self.SaveGameObject`)
      (:`Is Valid`
        _)
      (:`Is Not Valid`
        (bind _returnvalue (`GameplayStatics.LoadGameFromSlot` (`self.SaveSlotName`)))
        (bind _asbp_player_save_game (cast `/Game/Misc/SavingAndLoading/BP_PlayerSaveGame` _returnvalue))
        (set `self.SaveGameObject` _asbp_player_save_game)))
    (set `self.Settings` (`/Game/Misc/SavingAndLoading/BP_PlayerSaveGame.SavedSettings` _savegameobject))
    (set `/Game/ThirdPersonBP/Blueprints/ThirdPersonCharacter.CollectedBodyParts` (`/Game/Misc/SavingAndLoading/BP_PlayerSaveGame.SavedBodyParts` _savegameobject) _characterref)
    (`/Game/ThirdPersonBP/Blueprints/ThirdPersonCharacter.LoadBodyParts` _characterref)
    (set `self.LevelTags` (`/Game/Misc/SavingAndLoading/BP_PlayerSaveGame.SavedLevelTags` _savegameobject))
    (set `/Game/Misc/Memories/BP_Component_MemoryCounter.FoundMemories` (`/Game/Misc/SavingAndLoading/BP_PlayerSaveGame.SavedMemories` _savegameobject) (`/Game/ThirdPersonBP/Blueprints/ThirdPersonCharacter.MemoryCounter` _characterref))
    (bind _result (`BlueprintSetLibrary.Set_ToArray` (`self.CurrentlyLoadedLevels`)))
    (bind _result_2 (`BlueprintSetLibrary.Set_ToArray` (`/Game/Misc/SavingAndLoading/BP_PlayerSaveGame.SavedLoadedSubLevels` _savegameobject)))
    (`self.OnGameLoaded` _result _result_2 (`/Game/Misc/SavingAndLoading/BP_PlayerSaveGame.SavedLocation` _savegameobject) (`/Game/Misc/SavingAndLoading/BP_PlayerSaveGame.SavedRotation` _savegameobject) (`/Game/Misc/SavingAndLoading/BP_PlayerSaveGame.SavedControllerRotation` _savegameobject))
    (return)))

(fn `RegisterTag`
  (params (`Level Name` :type Name) (Tag :type String))
  (locals (localArray :type "Array of String"))
  (bind _leveltags (`self.LevelTags`))
  (bind (_value _returnvalue) (`BlueprintMapLibrary.Map_Find` _leveltags `Level Name`))
  (if _returnvalue
    (set `local.localArray` (`.Tags_3_AC2B457843A0A54F6BC1A799293853A6` (break `/Game/Misc/SavingAndLoading/STR_AreaTags` _value)))
    (`KismetArrayLibrary.Array_AddUnique` (`local.localArray`) Tag)
    (`BlueprintMapLibrary.Map_Add` _leveltags `Level Name` (make `/Game/Misc/SavingAndLoading/STR_AreaTags` (`local.localArray`)))
    (return)
    (else
      (`BlueprintMapLibrary.Map_Add` _leveltags `Level Name` (make `/Game/Misc/SavingAndLoading/STR_AreaTags` (`|MakeArray` Tag)))
      (return))))

(fn `SaveGame`
  (returns (`Success?` :type Boolean))
  (bind _savegameobject (`self.SaveGameObject`))
  (bind _characterref (`self.CharacterRef`))
  (bind _characterref_2 (`self.CharacterRef`))
  (`/Engine/EditorBlueprintResources/StandardMacros.IsValid` (`self.SaveGameObject`)
    (:`Is Valid`
      _)
    (:`Is Not Valid`
      (bind _returnvalue (`GameplayStatics.CreateSaveGameObject` "/Game/Misc/SavingAndLoading/BP_PlayerSaveGame.BP_PlayerSaveGame_C"))
      (set `self.SaveGameObject` _returnvalue)))
  (set `/Game/Misc/SavingAndLoading/BP_PlayerSaveGame.SavedLocation` (`Actor.K2_GetActorLocation` _characterref_2) _savegameobject)
  (set `/Game/Misc/SavingAndLoading/BP_PlayerSaveGame.SavedRotation` (`Actor.K2_GetActorRotation` _characterref_2) _savegameobject)
  (set `/Game/Misc/SavingAndLoading/BP_PlayerSaveGame.SavedControllerRotation` (`Controller.GetControlRotation` (`Pawn.GetController` _characterref_2)) _savegameobject)
  (set `/Game/Misc/SavingAndLoading/BP_PlayerSaveGame.SavedLoadedSubLevels` (`self.CurrentlyLoadedLevels`) _savegameobject)
  (set `/Game/Misc/SavingAndLoading/BP_PlayerSaveGame.SavedSettings` (`self.Settings`) _savegameobject)
  (set `/Game/Misc/SavingAndLoading/BP_PlayerSaveGame.SavedMemories` (`/Game/Misc/Memories/BP_Component_MemoryCounter.FoundMemories` (`/Game/ThirdPersonBP/Blueprints/ThirdPersonCharacter.MemoryCounter` _characterref)) _savegameobject)
  (set `/Game/Misc/SavingAndLoading/BP_PlayerSaveGame.SavedLevelTags` (`self.LevelTags`) _savegameobject)
  (set `/Game/Misc/SavingAndLoading/BP_PlayerSaveGame.SavedBodyParts` (`/Game/ThirdPersonBP/Blueprints/ThirdPersonCharacter.CollectedBodyParts` _characterref) _savegameobject)
  (bind _returnvalue_2 (`GameplayStatics.SaveGameToSlot` (`self.SaveGameObject`) (`self.SaveSlotName`)))
  (return _returnvalue_2))