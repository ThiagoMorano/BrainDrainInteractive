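; Box trigger volume that streams a list of levels in when the player enters and out on exit, notifying an optional connected door.
; Paired DoOnce gates and conditions from BpC_Saving guard both directions, and each change is recorded in that component.
; It can optionally blend sky sphere and skylight to a new preset via timeline.
; As first volume in a new game, it loads at BeginPlay and moves the player to a PlayerStart.
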(event `self.ReceiveBeginPlay`
  (if (`self.LoadAsFirst?`)
    (if (not (`/Game/Misc/SavingAndLoading/BP_GameInstance.IsLoadedGame?` (cast `/Game/Misc/SavingAndLoading/BP_GameInstance` (`GameplayStatics.GetGameInstance`) :!pure true)))
      (`self.LoadAsFirst`))))

(event `self.Box.OnComponentBeginOverlap`
  (params (OverlappedComponent :type "PrimitiveComponent Object Reference") (OtherActor :type "Actor Object Reference") (OtherComp :type "PrimitiveComponent Object Reference") (OtherBodyIndex :type Integer) (bFromSweep :type Boolean) (SweepResult :type "HitResult Structure (by ref)"))
  (bind _connecteddoor (`self.ConnectedDoor`))
  (bind _connecteddoor_2 (`self.ConnectedDoor`))
  (if (== OtherActor (`GameplayStatics.GetPlayerCharacter` 0))
    (if (not (`/Game/Misc/SavingAndLoading/BpC_Saving.HasLoadedAnyOfLevels?` (`self.GetComponentByClass` OtherActor "/Game/Misc/SavingAndLoading/BpC_Saving.BpC_Saving_C") (`self.DoNotLoadIfLoaded`)))
      (`/Engine/EditorBlueprintResources/StandardMacros.DoOnce` false :!label _label
        (:`Completed`
          (set `self.CurrentIndex` 0)
          (`|ExecutionSequence`
            (:`then_0`
              (`self.LoadAllLevels` true
                (:`Finished`
                  (set `self.CurrentIndex` 0)
                  (`/Engine/EditorBlueprintResources/StandardMacros.IsValid` _connecteddoor
                    (:`Is Valid`
                      (`KismetSystemLibrary.Delay` 0.2)
                      (`/Game/Misc/Door/BP_Door.OnLevelLoaded` _connecteddoor))))))
            (:`then_1`
              (goto _label_3 :!via `Reset`))
            (:`then_2`
              (if (`self.ChangeSkyOnEnter?`)
                (`self.ChangeSky`))))))
      (else
        (goto _label_3 :!via `Reset`)))))

(event `self.Box.OnComponentEndOverlap`
  (params (OverlappedComponent :type "PrimitiveComponent Object Reference") (OtherActor :type "Actor Object Reference") (OtherComp :type "PrimitiveComponent Object Reference") (OtherBodyIndex :type Integer))
  (bind _connecteddoor (`self.ConnectedDoor`))
  (if (== OtherActor (`GameplayStatics.GetPlayerCharacter` 0))
    (bind _asbp_rolling_head (cast `/Game/RollingBP/Blueprints/BP_RollingHead` OtherActor)
      (:`then`
        (if (not (`/Game/RollingBP/Blueprints/BP_RollingHead.Unpossessing?` _asbp_rolling_head))
          (if (and (!= (`self.OnlyUnloadIfLoaded`) "None") (not (`/Game/Misc/SavingAndLoading/BpC_Saving.HasLoadedLevel?` (`self.GetComponentByClass` OtherActor "/Game/Misc/SavingAndLoading/BpC_Saving.BpC_Saving_C") (`self.OnlyUnloadIfLoaded`)))) :!label _label_2
            (goto _label :!via `Reset`)
            (else
              (`/Engine/EditorBlueprintResources/StandardMacros.DoOnce` false :!label _label_3
                (:`Completed`
                  (set `self.CurrentIndex` 0)
                  (`|ExecutionSequence`
                    (:`then_0`
                      (`self.LoadAllLevels` false
                        (:`Finished`
                          (set `self.CurrentIndex` 0)
                          (`/Engine/EditorBlueprintResources/StandardMacros.IsValid` _connecteddoor
                            (:`Is Valid`
                              (`/Game/Misc/Door/BP_Door.OnLevelUnloaded` _connecteddoor))))))
                    (:`then_1`
                      (goto _label :!via `Reset`)))))))))
      (:`CastFailed`
        (goto _label_2)))))

(event `LoadAsFirst`
  (bind _returnvalue (`GameplayStatics.GetPlayerCharacter` 0))
  (`self.SetActorHiddenInGame` (`GameplayStatics.GetPlayerCharacter` 0) true)
  (if (`self.ChangeSkyOnEnter?`)
    (`self.FetchOldSkyData`)
    (`self.SetSkyValues` 1.0))
  (`self.LoadAllLevels` true
    (:`Finished`
      (bind _outactors (`GameplayStatics.GetAllActorsOfClass` "/Script/Engine.PlayerStart"))
      (`self.K2_SetActorLocation` _returnvalue (`self.K2_GetActorLocation` (`|GetArrayItem` _outactors)) false false)
      (`KismetSystemLibrary.Delay` 0.2)
      (`self.SetActorHiddenInGame` _returnvalue false))))

(event `ChangeSky`
  (`self.FetchOldSkyData`)
  (set `/Engine/EngineSky/BP_Sky_Sphere.Colors determined by sun position` (`.ColorsDeterminedBySun?_30_902CDFBA46C1B01782DE2BACFB5E1EED` (break `/Game/Misc/LevelStreaming/STR_SkyInfo` (`self.NewSky`))) (`self.GetSkyActor`))
  (bind (_direction _percent) (`Timeline|SkyLerp` :!via `PlayFromStart`)
    (:`Update`
      (`self.SetSkyValues` _percent))))

(fn `FetchOldSkyData`
  (bind _out (`self.GetSkyLight`))
  (bind _out_2 (`self.GetSkyActor`))
  (bind _lightcomponent (`SkyLight.LightComponent` _out))
  (set `self.OldSky` (make `/Game/Misc/LevelStreaming/STR_SkyInfo` (`/Engine/EngineSky/BP_Sky_Sphere.Colors determined by sun position` _out_2) (`/Engine/EngineSky/BP_Sky_Sphere.Sun brightness` _out_2) (`/Engine/EngineSky/BP_Sky_Sphere.Cloud speed` _out_2) (`/Engine/EngineSky/BP_Sky_Sphere.Cloud opacity` _out_2) (`/Engine/EngineSky/BP_Sky_Sphere.Stars brightness` _out_2) (`/Engine/EngineSky/BP_Sky_Sphere.Sun height` _out_2) (`/Engine/EngineSky/BP_Sky_Sphere.Horizon Falloff` _out_2) (`/Engine/EngineSky/BP_Sky_Sphere.Zenith Color` _out_2) (`/Engine/EngineSky/BP_Sky_Sphere.Horizon color` _out_2) (`/Engine/EngineSky/BP_Sky_Sphere.Cloud color` _out_2) (`/Engine/EngineSky/BP_Sky_Sphere.Overall Color` _out_2) (`LightComponentBase.Intensity` _lightcomponent) (`LightComponentBase.GetLightColor` _lightcomponent) (`self.K2_GetActorRotation` _out))))

(fn `GetSkyActor`
  (returns (Out :type "/Engine/EngineSky/BP_Sky_Sphere Object Reference"))
  (`/Engine/EditorBlueprintResources/StandardMacros.IsValid` (`self.SkyRef`)
    (:`Is Valid`
      _)
    (:`Is Not Valid`
      (bind _outactors (`GameplayStatics.GetAllActorsOfClass` "/Engine/EngineSky/BP_Sky_Sphere.BP_Sky_Sphere_C"))
      (bind _output_get (set `self.SkyRef` (`|GetArrayItem` _outactors)))))
  (return _output_get))

(fn `GetSkyLight`
  (returns (Out :type "SkyLight Object Reference"))
  (`/Engine/EditorBlueprintResources/StandardMacros.IsValid` (`self.LightRef`)
    (:`Is Valid`
      _)
    (:`Is Not Valid`
      (bind _outactors (`GameplayStatics.GetAllActorsOfClass` "/Script/Engine.SkyLight"))
      (set `self.LightRef` (`|GetArrayItem` _outactors))))
  (return (`self.LightRef`)))

(fn `SetSkyValues`
  (params (Percent :type "Float (double-precision)"))
  (bind _out (`self.GetSkyActor`))
  (bind _out_2 (`self.GetSkyLight`))
  (bind (_colorsdeterminedbysun_ _sunbrightness _cloudspeed _cloudopacity _starsbrightness _sunheight _horizonfalloff _zenithcolor _horizoncolor _cloudcolor _overallcolor _lightintensity _lightcolor _lightrotation) (break `/Game/Misc/LevelStreaming/STR_SkyInfo` (`self.OldSky`)))
  (bind (_colorsdeterminedbysun__2 _sunbrightness_2 _cloudspeed_2 _cloudopacity_2 _starsbrightness_2 _sunheight_2 _horizonfalloff_2 _zenithcolor_2 _horizoncolor_2 _cloudcolor_2 _overallcolor_2 _lightintensity_2 _lightcolor_2 _lightrotation_2) (break `/Game/Misc/LevelStreaming/STR_SkyInfo` (`self.NewSky`)))
  (bind _lightcomponent (`SkyLight.LightComponent` _out_2))
  (set `/Engine/EngineSky/BP_Sky_Sphere.Sun height` (`KismetMathLibrary.Lerp` _sunheight _sunheight_2 Percent) _out)
  (set `/Engine/EngineSky/BP_Sky_Sphere.Cloud speed` (`KismetMathLibrary.Lerp` _cloudspeed _cloudspeed_2 Percent) _out)
  (set `/Engine/EngineSky/BP_Sky_Sphere.Cloud opacity` (`KismetMathLibrary.Lerp` _cloudopacity _cloudopacity_2 Percent) _out)
  (set `/Engine/EngineSky/BP_Sky_Sphere.Overall Color` (`KismetMathLibrary.LinearColorLerp` _overallcolor _overallcolor_2 Percent) _out)
  (set `/Engine/EngineSky/BP_Sky_Sphere.Cloud color` (`KismetMathLibrary.LinearColorLerp` _cloudcolor _cloudcolor_2 Percent) _out)
  (set `/Engine/EngineSky/BP_Sky_Sphere.Zenith Color` (`KismetMathLibrary.LinearColorLerp` _zenithcolor _zenithcolor_2 Percent) _out)
  (set `/Engine/EngineSky/BP_Sky_Sphere.Horizon color` (`KismetMathLibrary.LinearColorLerp` _horizoncolor _horizoncolor_2 Percent) _out)
  (set `/Engine/EngineSky/BP_Sky_Sphere.Sun brightness` (`KismetMathLibrary.Lerp` _sunbrightness _sunbrightness_2 Percent) _out)
  (set `/Engine/EngineSky/BP_Sky_Sphere.Stars brightness` (`KismetMathLibrary.Lerp` _starsbrightness _starsbrightness_2 Percent) _out)
  (set `/Engine/EngineSky/BP_Sky_Sphere.Horizon Falloff` (`KismetMathLibrary.Lerp` _horizonfalloff _horizonfalloff_2 Percent) _out)
  (`SkyLightComponent.SetIntensity` _lightcomponent (`KismetMathLibrary.Lerp` _lightintensity _lightintensity_2 Percent))
  (`SkyLightComponent.SetLightColor` _lightcomponent (`KismetMathLibrary.LinearColorLerp` _lightcolor _lightcolor_2 Percent))
  (`self.K2_SetActorRotation` _out_2 (`KismetMathLibrary.RLerp` _lightrotation _lightrotation_2 Percent) false)
  (`/Engine/EngineSky/BP_Sky_Sphere.RefreshMaterial` _out))

(fn `UserConstructionScript`
  (`BoxComponent.SetBoxExtent` (`self.Box`) (`self.BoxExtent`) true))