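; Component that tracks which memories have been found in each area and looks up the memory content to show.
; RegisterMemory stores ID and order number pairs in a per-area map, which lookups scan for found state or the next number.
; FetchMemoryToShow uses the order number as a one-based index into the area's memory list, decoupling content from ID.
; The next-number query returns -1 for areas with nothing registered.
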(fn `FetchMemoryToShow`
  (params (Area :type "/Game/Misc/Memories/ENUM_Areas Enum" :default "NewEnumerator0") (OrderNumber :type Integer))
  (returns (`Success?` :type Boolean) (Memory :type "/Game/Misc/Memories/STR_MemoryInfo Structure"))
  (bind (_value _returnvalue) (`BlueprintMapLibrary.Map_Find` (`self.MemoriesInAreas`) Area))
  (if _returnvalue
    (return true (`|GetArrayItem` (`.Memories_7_19742BB246DA7EBAACC018B7DEEC93E9` (break `/Game/Misc/Memories/STR_AreaMemories` _value)) (- OrderNumber 1)))
    (else
      (return false))))

(fn `GetNextNumberForArea`
  (params (Area :type "/Game/Misc/Memories/ENUM_Areas Enum" :default "NewEnumerator0"))
  (returns (Number :type Integer))
  (locals (localHighestOrder :type Integer))
  (bind _localhighestorder (`local.localHighestOrder`))
  (bind (_value _returnvalue) (`BlueprintMapLibrary.Map_Find` (`self.FoundMemories`) Area))
  (if _returnvalue
    (for _array_element (`.Memories_7_9C1922694303B60F52024E92A54B2D7C` (break `/Game/Misc/Memories/STR_MemoryIDsInArea` _value))
      (bind (_id _ordernumber) (break `/Game/Misc/Memories/STR_MemoryID` _array_element))
      (if (> _ordernumber _localhighestorder)
        (set `local.localHighestOrder` _ordernumber)))
    (return (+ _localhighestorder 1))
    (else
      (return -1))))

(fn `HasFoundMemory?`
  (params (Area :type "/Game/Misc/Memories/ENUM_Areas Enum" :default "NewEnumerator0") (ID :type Integer))
  (returns (`Found?` :type Boolean) (OrderNumber :type Integer))
  (locals (localFound :type Boolean) (localOrder :type Integer) (IdToFind :type Integer))
  (bind (_value _returnvalue) (`BlueprintMapLibrary.Map_Find` (`self.FoundMemories`) Area))
  (set `local.IdToFind` ID)
  (if _returnvalue
    (for _array_element (`.Memories_7_9C1922694303B60F52024E92A54B2D7C` (break `/Game/Misc/Memories/STR_MemoryIDsInArea` _value))
      (bind (_id _ordernumber) (break `/Game/Misc/Memories/STR_MemoryID` _array_element))
      (if (== _id (`local.IdToFind`))
        (set `local.localFound` true)
        (set `local.localOrder` _ordernumber)
        (break)))
    (return (`local.localFound`) (`local.localOrder`))
    (else
      (return false 0))))

(fn `RegisterMemory`
  (params (Area :type "/Game/Misc/Memories/ENUM_Areas Enum" :default "NewEnumerator0") (ID :type Integer) (OrderNumber :type Integer))
  (locals (localMemories :type "Array of /Game/Misc/Memories/STR_MemoryID Structure"))
  (bind _str_memoryid (make `/Game/Misc/Memories/STR_MemoryID` ID OrderNumber))
  (bind _foundmemories (`self.FoundMemories`))
  (bind _foundmemories_2 (`self.FoundMemories`))
  (if (`BlueprintMapLibrary.Map_Contains` _foundmemories Area)
    (set `local.localMemories` (`.Memories_7_9C1922694303B60F52024E92A54B2D7C` (break `/Game/Misc/Memories/STR_MemoryIDsInArea` (`BlueprintMapLibrary.Map_Find` _foundmemories Area))))
    (`KismetArrayLibrary.Array_Add` (`local.localMemories`) _str_memoryid)
    (`BlueprintMapLibrary.Map_Add` _foundmemories_2 Area (make `/Game/Misc/Memories/STR_MemoryIDsInArea` (`local.localMemories`)))
    (return)
    (else
      (`BlueprintMapLibrary.Map_Add` _foundmemories_2 Area (make `/Game/Misc/Memories/STR_MemoryIDsInArea` (`|MakeArray` _str_memoryid)))
      (return))))