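; BP_Memory is a collectible memory shard that appears facing the camera when the player enters its ShowArea.
; On first show, it registers with BP_Component_MemoryCounter for a per-area order number, so discovery order picks its texture.
; Camera look time accumulates on Tick, dissolving it at one threshold, or at another upon leaving; otherwise it hides again.
; Dissolves are registered in the counter, so previously dissolved memories destroy themselves on BeginPlay.
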(event `LoadMemoryExistence`
  ;[1 1 1] Load Memory Existence
  (if (`.Dissolve?` (`/Game/Misc/Memories/BP_Component_MemoryCounter.HasFoundMemory?` (`self.GetComponentByClass` (`self.Player`) "/Game/Misc/Memories/BP_Component_MemoryCounter.BP_Component_MemoryCounter_C") (`self.Area`) (`self.ID`)))
    (`self.K2_DestroyActor`)))

(event `self.ReceiveBeginPlay`
  (bind _shardsmesh (`self.ShardsMesh`))
  ;[1 1 1] Store a reference to the player on BEGIN PLAY
  (bind _asthird_person_character (cast `/Game/ThirdPersonBP/Blueprints/ThirdPersonCharacter` (`GameplayStatics.GetPlayerCharacter` 0)))
  (set `self.Player` _asthird_person_character)
  (`self.LoadMemoryExistence`)
  (`self.HideMemory`)
  (set `self.OriginalShardsRotation` (`SceneComponent.K2_GetComponentRotation` (`self.ShardsMesh`)))
  (set `self.MeshScale` (`SceneComponent.K2_GetComponentScale` (`self.ShardsMesh`)))
  (bind _returnvalue (`PrimitiveComponent.CreateDynamicMaterialInstance` _shardsmesh 0 (`PrimitiveComponent.GetMaterial` _shardsmesh 0) "None"))
  (bind _output_get (set `self.DynamicShardsMaterial` _returnvalue))
  (`MaterialInstanceDynamic.SetVectorParameterValue` _output_get "FringeColor" (select `/Game/Misc/Memories/ENUM_Areas` (`self.Area`) :`NewEnumerator0` (struct :`R` 0.658333 :`G` 0.374352 :`B` 0.164488 :`A` 1.0) :`NewEnumerator1` (struct :`R` 0.658333 :`G` 0.374352 :`B` 0.164488 :`A` 1.0) :`NewEnumerator2` (struct :`R` 0.228163 :`G` 0.400805 :`B` 0.658333 :`A` 1.0) :`NewEnumerator3` (struct :`R` 0.845833 :`G` 0.235966 :`B` 0.762542 :`A` 1.0) :`NewEnumerator4` (struct :`R` 0.658333 :`G` 0.374352 :`B` 0.164488 :`A` 1.0) :!type "LinearColor Structure")))

(event `OnFirstShow`
  (bind _area (`self.Area`))
  (bind _area_2 (`self.Area`))
  (bind _returnvalue (`self.GetComponentByClass` (`self.Player`) "/Game/Misc/Memories/BP_Component_MemoryCounter.BP_Component_MemoryCounter_C"))
  (bind (_found_ _ordernumber _dissolve_) (`/Game/Misc/Memories/BP_Component_MemoryCounter.HasFoundMemory?` _returnvalue _area_2 (`self.ID`)))
  (bind (_success_ _memory) (`/Game/Misc/Memories/BP_Component_MemoryCounter.FetchMemoryToShow` _returnvalue _area (`self.StoredOrderToUse`)))
  ;[1 1 1] On Memory First Shown
  (set `self.ShownBefore?` true)
  (`/Engine/EditorBlueprintResources/StandardMacros.IsValid` _returnvalue
    (:`Is Valid`
      (if _found_
        (if (not _dissolve_)
          (`MaterialInstanceDynamic.SetTextureParameterValue` (`self.DynamicShardsMaterial`) "BaseTexture" (`.MeshTexture_9_0815F2694C0200EB24321C9D90B604B2` (break `/Game/Misc/Memories/STR_MemoryInfo` (`.Memory` (`/Game/Misc/Memories/BP_Component_MemoryCounter.FetchMemoryToShow` _returnvalue (`self.Area`) _ordernumber))))))
        (else
          (bind _output_get (set `self.StoredOrderToUse` (`/Game/Misc/Memories/BP_Component_MemoryCounter.GetNextNumberForArea` _returnvalue _area_2)))
          (`/Game/Misc/Memories/BP_Component_MemoryCounter.RegisterMemory` _returnvalue _area (`self.ID`) _output_get)
          (if _success_
            (`MaterialInstanceDynamic.SetTextureParameterValue` (`self.DynamicShardsMaterial`) "BaseTexture" (`.MeshTexture_9_0815F2694C0200EB24321C9D90B604B2` (break `/Game/Misc/Memories/STR_MemoryInfo` _memory)))))))))

(event `DissolveMemory`
  ;[1 1 1] DissolveMemory
  (if (not (`self.Dissolved?`))
    (set `self.Dissolved?` true)
    (bind _success_ (`/Game/Misc/Memories/BP_Component_MemoryCounter.RegisterMemoryDissolve` (`self.GetComponentByClass` (`self.Player`) "/Game/Misc/Memories/BP_Component_MemoryCounter.BP_Component_MemoryCounter_C") (`self.Area`) (`self.ID`)))
    (if _success_
      (bind (_direction _dissolveamount) (`Timeline|DissolveTimeline` :!via `PlayFromStart`)
        (:`Update`
          (`MaterialInstanceDynamic.SetScalarParameterValue` (`self.DynamicShardsMaterial`) "DissolveAmount" _dissolveamount))
        (:`Finished`
          (`self.K2_DestroyActor`))))))

(event `self.ShowArea.OnComponentBeginOverlap`
  (params (OverlappedComponent :type "PrimitiveComponent Object Reference") (OtherActor :type "Actor Object Reference") (OtherComp :type "PrimitiveComponent Object Reference") (OtherBodyIndex :type Integer) (bFromSweep :type Boolean) (SweepResult :type "HitResult Structure (by ref)"))
  (bind _player (`self.Player`))
  ;[1 1 1] When player enters/leaves showArea, show/hide the memory
  (`/Engine/EditorBlueprintResources/StandardMacros.IsValid` _player
    (:`Is Valid`
      (if (== _player OtherActor)
        (if (not (`self.Dissolved?`))
          (if (not (`self.PlayerNearby?`))
            (`self.ShowMemory`)))))))

(event `self.ShowArea.OnComponentEndOverlap`
  (params (OverlappedComponent :type "PrimitiveComponent Object Reference") (OtherActor :type "Actor Object Reference") (OtherComp :type "PrimitiveComponent Object Reference") (OtherBodyIndex :type Integer))
  (bind _player (`self.Player`))
  ;[1 1 1] When player enters/leaves showArea, show/hide the memory
  (`/Engine/EditorBlueprintResources/StandardMacros.IsValid` _player
    (:`Is Valid`
      (if (== _player OtherActor)
        (if (not (`self.Dissolved?`))
          (if (`self.PlayerNearby?`)
            (if (>= (`self.LookAtTime`) (`self.TimeBeforeDissolveAtLeave`))
              (`self.DissolveMemory`)
              (else
                (`self.HideMemory`)))))))))

(event `self.ReceiveTick`
  (params (DeltaSeconds :type "Float (single-precision)"))
  ;[1 1 1] Fetch Look At Time On Tick
  (if (and (`self.PlayerNearby?`) (not (`self.Dissolved?`)))
    (if (`/Game/ThirdPersonBP/Blueprints/ThirdPersonCharacter.ActorInCameraView?` (`self.Player`) self (`self.ShardsMesh`) (`|MakeArray` "ObjectTypeQuery5" :!type "EObjectTypeQuery Enum"))
      (set `self.LookAtTime` (+ (`self.LookAtTime`) DeltaSeconds))
      (if (>= (`self.LookAtTime`) (`self.TimeBeforeDissolve`))
        (`self.DissolveMemory`)))))

(event `ShowMemory`
  ;[1 1 1] Show Memory
  (set `self.PlayerNearby?` true)
  (if (not (`self.ShownBefore?`))
    (`self.OnFirstShow`))
  (`SceneComponent.SetWorldScale3D` (`self.ShardsMesh`) (0.0 0.0 0.0))
  (`self.RotateToFaceCamera`)
  (`SceneComponent.SetVisibility` (`self.ShardsMesh`) true false)
  (`ActorComponent.Deactivate` (`self.ParticleShards`))
  (bind (_direction _percentagescale _opacity) (`Timeline|ShowStuff` :!label _label)
    (:`Update`
      (`SceneComponent.SetWorldScale3D` (`self.ShardsMesh`) (* (`self.MeshScale`) _percentagescale))
      (`MaterialInstanceDynamic.SetScalarParameterValue` (`self.DynamicShardsMaterial`) "Opacity" _opacity))
    (:`Finished`
      (switch `ETimelineDirection` _direction
        (:`Backward`
          (`SceneComponent.SetVisibility` (`self.ShardsMesh`) false false)
          (`ActorComponent.Activate` (`self.ParticleShards`) false))))))

(event `HideMemory`
  ;[1 1 1] Show Memory
  (set `self.PlayerNearby?` false)
  (set `self.LookAtTime` 0.0)
  (goto _label :!via `Reverse`))

(fn `RotateToFaceCamera`
  (bind _shardsmesh (`self.ShardsMesh`))
  (`SceneComponent.K2_SetWorldRotation` _shardsmesh (`KismetMathLibrary.ComposeRotators` (`KismetMathLibrary.MakeRotator` (.roll (`SceneComponent.K2_GetComponentRotation` _shardsmesh)) (.pitch (`SceneComponent.K2_GetComponentRotation` _shardsmesh)) (+ (.yaw (`KismetMathLibrary.FindLookAtRotation` (`SceneComponent.K2_GetComponentLocation` (`self.ShowArea`)) (`SceneComponent.K2_GetComponentLocation` (`/Game/ThirdPersonBP/Blueprints/ThirdPersonCharacter.FollowCamera` (`self.Player`))))) 270.0)) (`self.OriginalShardsRotation`)) false false))

(fn `UserConstructionScript`)