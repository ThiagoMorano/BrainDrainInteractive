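; BP_FixedHubMemory is a memory prop, apparently placed in the hub, that shows only when the player has a required body part.
; On BeginPlay it passes the player character's BpC_BodyParts component to Update, which hides the actor if RequiredBodyPart is missing.
; The construction script creates a dynamic material on MemoryMesh and sets its Texture parameter to the Memory image, so each instance can display its own picture.
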(event `self.ReceiveBeginPlay`
  (`self.Update` (`self.GetComponentByClass` (`GameplayStatics.GetPlayerCharacter` 0) "/Game/ThirdPersonBP/Blueprints/BodyPartAbilities/BpC_BodyParts.BpC_BodyParts_C")))

(event `Update`
  (params (`Body Parts` :type "/Game/ThirdPersonBP/Blueprints/BodyPartAbilities/BpC_BodyParts Object Reference"))
  (`/Engine/EditorBlueprintResources/StandardMacros.IsValid` `Body Parts`
    (:`Is Valid`
      (`self.SetActorHiddenInGame` (not (`/Game/ThirdPersonBP/Blueprints/BodyPartAbilities/BpC_BodyParts.HasBodyPart?` `Body Parts` (`self.RequiredBodyPart`)))))))

(fn `UserConstructionScript`
  (bind _memorymesh (`self.MemoryMesh`))
  (bind _returnvalue (`PrimitiveComponent.CreateDynamicMaterialInstance` _memorymesh 0 (`PrimitiveComponent.GetMaterial` _memorymesh 0) "None"))
  (bind _output_get (set `self.DynamicMaterial` _returnvalue))
  (`MaterialInstanceDynamic.SetTextureParameterValue` _output_get "Texture" (`self.Memory`)))