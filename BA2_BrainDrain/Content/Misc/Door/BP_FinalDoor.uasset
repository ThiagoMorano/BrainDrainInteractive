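; BP_FinalDoor is a door that swings open once, when the player character enters its trigger collision.
; Opening sets a flag against retriggering, asks the sound manager to fade out and pause the music, then plays the opening effect after a short delay.
; In parallel, a timeline lerps the door mesh's relative rotation from its original to a yaw-offset target.
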(event `self.OpenDoorCollision.OnComponentBeginOverlap`
  (params (OverlappedComponent :type "PrimitiveComponent Object Reference") (OtherActor :type "Actor Object Reference") (OtherComp :type "PrimitiveComponent Object Reference") (OtherBodyIndex :type Integer) (bFromSweep :type Boolean) (SweepResult :type "HitResult Structure (by ref)"))
  (bind _returnvalue (`GameplayStatics.GetPlayerCharacter` 0))
  (if (`self.Open?`)
    _
    (elif (== OtherActor _returnvalue)
      (set `self.Player` _returnvalue)
      (`self.OpenDoor`))))

(event `OpenDoor`
  (bind _out (`/Game/Misc/Sound/LIB_Sound.GetSoundManager`))
  (set `self.Open?` true)
  (`|ExecutionSequence`
    (:`then_0`
      (`/Game/Misc/Sound/BP_SoundManager.PauseMusic` _out 4.0 20.0)
      (`KismetSystemLibrary.Delay` 1.0)
      (`/Game/Misc/Sound/BP_SoundManager.PlayEffect` _out "/Game/Misc/Sound/Effects/Objects/SFX_Door_Opening_WithFade.SFX_Door_Opening_WithFade" true (`self.K2_GetActorLocation`) 0.0 1.0 1.0))
    (:`then_1`
      (set `self.OriginalRotation` (`SceneComponent.RelativeRotation` (`self.DoorMesh`)))
      (set `self.FinalRotation` (`KismetMathLibrary.ComposeRotators` (`self.OriginalRotation`) (`KismetMathLibrary.MakeRotator` 0.0 0.0 (`self.SwingOpenYaw`))))
      (bind (_direction _percent) (`Timeline|SwingOpen` :!via `PlayFromStart`)
        (:`Update`
          (`SceneComponent.K2_SetRelativeRotation` (`self.DoorMesh`) (`KismetMathLibrary.RLerp` (`self.OriginalRotation`) (`self.FinalRotation`) _percent true) false false))))))

(fn `UserConstructionScript`)