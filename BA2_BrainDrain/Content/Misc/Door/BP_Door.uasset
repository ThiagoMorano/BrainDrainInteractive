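; BP_Door is a two-leaf door that opens when the player with the required body part enters its open area, waiting for its linked streaming volume's level to load.
; A timeline drives leaf rotation and emissive glow on dynamic materials, accompanied by delayed camera shake and sound.
; The close area reverses it, then swaps streamed levels after a delay, and saves if the player lacks the next body part.
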(event `self.ReceiveBeginPlay`
  (bind _framemesh (`self.FrameMesh`))
  (bind _lefthalfmesh (`self.LeftHalfMesh`))
  (bind _righthalfmesh (`self.RightHalfMesh`))
  (bind _connectedstreamingvolume (`self.ConnectedStreamingVolume`))
  ;[1 1 1] Begin Play
  (`/Engine/EditorBlueprintResources/StandardMacros.IsValid` _connectedstreamingvolume
    (:`Is Valid`
      (set `/Game/Misc/LevelStreaming/BP_CustomStreamingVolume.ConnectedDoor` self _connectedstreamingvolume)
      (set `self.Loaded?` false))
    (:`Is Not Valid`
      (set `self.Loaded?` true)))
  (bind _returnvalue (`PrimitiveComponent.CreateDynamicMaterialInstance` _framemesh 0 (`PrimitiveComponent.GetMaterial` _framemesh 0) "None"))
  (`KismetArrayLibrary.Array_Add` (`self.MaterialInstances`) _returnvalue)
  (bind _returnvalue_2 (`PrimitiveComponent.CreateDynamicMaterialInstance` _lefthalfmesh 0 (`PrimitiveComponent.GetMaterial` _lefthalfmesh 0) "None"))
  (`KismetArrayLibrary.Array_Add` (`self.MaterialInstances`) _returnvalue_2)
  (bind _returnvalue_3 (`PrimitiveComponent.CreateDynamicMaterialInstance` _righthalfmesh 0 (`PrimitiveComponent.GetMaterial` _righthalfmesh 0) "None"))
  (`KismetArrayLibrary.Array_Add` (`self.MaterialInstances`) _returnvalue_3)
  (`self.SetGlowStrength` (`self.ClosedGlowAmount`)))

(event `self.OpenArea.OnComponentBeginOverlap`
  (params (OverlappedComponent :type "PrimitiveComponent Object Reference") (OtherActor :type "Actor Object Reference") (OtherComp :type "PrimitiveComponent Object Reference") (OtherBodyIndex :type Integer) (bFromSweep :type Boolean) (SweepResult :type "HitResult Structure (by ref)"))
  (bind _returnvalue (`self.GetComponentByClass` OtherActor "/Game/ThirdPersonBP/Blueprints/BodyPartAbilities/BpC_BodyParts.BpC_BodyParts_C"))
  (if (not (`self.Open?`))
    (if (== OtherActor (`GameplayStatics.GetPlayerCharacter` 0))
      (`/Engine/EditorBlueprintResources/StandardMacros.IsValid` _returnvalue
        (:`Is Valid`
          (if (`/Game/ThirdPersonBP/Blueprints/BodyPartAbilities/BpC_BodyParts.HasBodyPart?` _returnvalue (`self.RequiredBodyPart`))
            (if (`self.Loaded?`)
              (`self.Open Door`)
              (else
                (set `self.ShouldOpen?` true)))))))))

(event `Open Door`
  (bind _openrotation (`self.OpenRotation`))
  (bind _returnvalue (`SceneComponent.K2_GetComponentLocation` (`self.FrameMesh`)))
  (set `self.Open?` true)
  (`|ExecutionSequence`
    (:`then_0`
      (bind (_direction _glowpercent _rotationpercent) (`Timeline|OpenTimeline` :!via `PlayFromStart` :!label _label)
        (:`Update`
          (`self.SetGlowStrength` (`KismetMathLibrary.Lerp` (`self.ClosedGlowAmount`) (`self.OpenGlowAmount`) _glowpercent))
          (`SceneComponent.K2_SetRelativeRotation` (`self.LeftHalfMesh`) (`KismetMathLibrary.MakeRotator` 0.0 0.0 (`KismetMathLibrary.Lerp` 0.0 (* _openrotation -1.0) _rotationpercent)) false false)
          (`SceneComponent.K2_SetRelativeRotation` (`self.RightHalfMesh`) (`KismetMathLibrary.MakeRotator` 0.0 0.0 (`KismetMathLibrary.Lerp` 0.0 _openrotation _rotationpercent)) false false))))
    (:`then_1`
      (`KismetSystemLibrary.Delay` 0.6)
      (`GameplayStatics.PlayWorldCameraShake` "/Game/Misc/Door/BP_Door_CameraShake.BP_Door_CameraShake_C" _returnvalue 100.0 5000.0))
    (:`then_2`
      (`KismetSystemLibrary.Delay` 0.7)
      (`/Game/Misc/Sound/BP_SoundManager.PlayEffect` (`/Game/Misc/Sound/LIB_Sound.GetSoundManager`) "/Game/Misc/Sound/Effects/Objects/SFX_Door_Opening_WithFade.SFX_Door_Opening_WithFade" true _returnvalue 0.1 1.0 1.4))))

(event `CloseDoor`
  (bind _unloadlevel (`self.UnloadLevel`))
  (bind _loadlevel (`self.LoadLevel`))
  (bind _returnvalue (`SceneComponent.K2_GetComponentLocation` (`self.FrameMesh`)))
  (bind _returnvalue_2 (`self.GetComponentByClass` (`GameplayStatics.GetPlayerCharacter` 0) "/Game/Misc/SavingAndLoading/BpC_Saving.BpC_Saving_C"))
  (if (`self.Open?`)
    (set `self.Open?` false)
    (`|ExecutionSequence`
      (:`then_0`
        (goto _label :!via `ReverseFromEnd`))
      (:`then_1`
        (`KismetSystemLibrary.Delay` 0.6)
        (`GameplayStatics.PlayWorldCameraShake` "/Game/Misc/Door/BP_Door_CameraShake.BP_Door_CameraShake_C" _returnvalue 100.0 5000.0))
      (:`then_2`
        (`KismetSystemLibrary.Delay` 0.7)
        (`/Game/Misc/Sound/BP_SoundManager.PlayEffect` (`/Game/Misc/Sound/LIB_Sound.GetSoundManager`) "/Game/Misc/Sound/Effects/Objects/SFX_Door_Opening_WithFade.SFX_Door_Opening_WithFade" true _returnvalue 0.1 0.9 0.9))
      (:`then_3`
        (`KismetSystemLibrary.Delay` 3.0)
        (if (!= _unloadlevel "None")
          (`/Game/Misc/SavingAndLoading/BpC_Saving.AdjustLoadedLevels` _returnvalue_2 _unloadlevel false)
          (`GameplayStatics.UnloadStreamLevel` _unloadlevel))
        (if (!= _loadlevel "None")
          (`/Game/Misc/SavingAndLoading/BpC_Saving.AdjustLoadedLevels` _returnvalue_2 _loadlevel true)
          (`GameplayStatics.LoadStreamLevel` _loadlevel true))))))

(event `OnLevelLoaded`
  (set `self.Loaded?` true)
  (if (and (`self.ShouldOpen?`) (not (`self.Open?`)))
    (`self.Open Door`)))

(event `self.CloseArea.OnComponentBeginOverlap`
  (params (OverlappedComponent :type "PrimitiveComponent Object Reference") (OtherActor :type "Actor Object Reference") (OtherComp :type "PrimitiveComponent Object Reference") (OtherBodyIndex :type Integer) (bFromSweep :type Boolean) (SweepResult :type "HitResult Structure (by ref)"))
  (bind _returnvalue (`self.GetComponentByClass` OtherActor "/Game/ThirdPersonBP/Blueprints/BodyPartAbilities/BpC_BodyParts.BpC_BodyParts_C"))
  (bind _returnvalue_2 (`self.GetComponentByClass` OtherActor "/Game/Misc/SavingAndLoading/BpC_Saving.BpC_Saving_C"))
  (if (`self.Open?`)
    (if (== OtherActor (`GameplayStatics.GetPlayerCharacter` 0))
      (`/Engine/EditorBlueprintResources/StandardMacros.IsValid` _returnvalue
        (:`Is Valid`
          (`self.CloseDoor`)
          (`/Engine/EditorBlueprintResources/StandardMacros.IsValid` _returnvalue_2
            (:`Is Valid`
              (if (not (`/Game/ThirdPersonBP/Blueprints/BodyPartAbilities/BpC_BodyParts.HasBodyPart?` _returnvalue (cast `/Game/Misc/SavingAndLoading/ENUM_BodyParts` (+ (`self.RequiredBodyPart`) 1))))
                (`/Game/Misc/SavingAndLoading/BpC_Saving.SaveGame` _returnvalue_2)))))))))

(event `OnLevelUnloaded`
  (set `self.Loaded?` false))

(fn `SetGlowStrength`
  (params (Value :type "Float (double-precision)"))
  (for _array_element (`self.MaterialInstances`)
    (`MaterialInstanceDynamic.SetScalarParameterValue` _array_element "EmissiveAmount" Value))
  (return))

(fn `UserConstructionScript`)