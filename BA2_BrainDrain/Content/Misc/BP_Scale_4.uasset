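; BP_Scale_4 is a balance scale with a tilting arm and two bowls.
; Each Tick applies ScaleRotation as the arm's roll and moves the bowls to their anchor components' world locations, without copying rotation.
; LerpScaletonewRotation plays a timeline that writes its raw value to ScaleRotation, leaving the NewRotation lerp unused.
; AddRotationtoScale only stores the starting angle and plays a timeline with no connected output.
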(event `self.ReceiveTick`
  (params (DeltaSeconds :type "Float (single-precision)"))
  (bind _arm (`self.Arm`))
  (bind (_relativerotation_roll _relativerotation_pitch _relativerotation_yaw) (`KismetMathLibrary.BreakRotator` (`SceneComponent.RelativeRotation` _arm)))
  (`SceneComponent.K2_SetRelativeRotation` _arm (`KismetMathLibrary.MakeRotator` (`self.ScaleRotation`) _relativerotation_pitch _relativerotation_yaw) false false)
  (`SceneComponent.K2_SetWorldLocation` (`self.LeftBowl`) (`SceneComponent.K2_GetComponentLocation` (`self.LeftBowlPosition`)) false false)
  (`SceneComponent.K2_SetWorldLocation` (`self.RightBowl`) (`SceneComponent.K2_GetComponentLocation` (`self.RightBowlPosition`)) false false))

(event `Lerp Scale to new Rotation`
  (params (`New Rotation` :type "Float (double-precision)"))
  (set `self.Starting Angle` (`self.ScaleRotation`))
  (bind (_direction _rotation_value) (`Timeline|Lerp Rotation` :!via `PlayFromStart`)
    (:`Update`
      (set `self.ScaleRotation` _rotation_value))))

(event `Add Rotation to Scale`
  (params (`Angles to sum` :type "Float (double-precision)"))
  (set `self.Starting Angle` (`self.ScaleRotation`))
  (`Timeline|Timeline_0` :!via `PlayFromStart`))

(fn `UserConstructionScript`)